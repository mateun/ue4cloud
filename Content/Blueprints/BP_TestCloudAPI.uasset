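; Test actor that exercises the CloudAPIFunctionLibrary on BeginPlay.
; It initializes the library with hardcoded placeholder credentials, then fetches raw JSON from a collection using an empty name and prints it.
; It then fills a MySaveGame with sample values across many variable types, saves it to the cloud under a fixed key and prints the result.
; MyStructTestFunc is an uncalled stub that returns a constant string.
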(event `self.ReceiveBeginPlay`
  (bind _output_get (set `self.CloudAPIFuncLib` (`CloudAPIFunctionLibrary.Initialize` "/Script/CloudPlugin.CloudAPIFunctionLibrary" "foo" "bar")))
  (bind _returnvalue (`CloudAPIFunctionLibrary.GetRawJsonDataFromCollection` _output_get ""))
  (`KismetSystemLibrary.PrintText` (`KismetTextLibrary.Conv_StringToText` _returnvalue))
  (bind _returnvalue_2 (`GameplayStatics.CreateSaveGameObject` "/Game/Blueprints/MySaveGame.MySaveGame_C"))
  (bind _asmy_save_game (cast `/Game/Blueprints/MySaveGame` _returnvalue_2))
  ;[1 1 1] Set the values to the SaveGame
  (`|ExecutionSequence`
    (:`then_0`
      (set `/Game/Blueprints/MySaveGame.hp` 10 _asmy_save_game))
    (:`then_1`
      (set `/Game/Blueprints/MySaveGame.playerScore` 258 _asmy_save_game))
    (:`then_2`
      (set `/Game/Blueprints/MySaveGame.playerName` "Franz" _asmy_save_game))
    (:`then_3`
      (set `/Game/Blueprints/MySaveGame.MyByteVar` 255 _asmy_save_game))
    (:`then_4`
      (set `/Game/Blueprints/MySaveGame.MyFloatVar` 12.56 _asmy_save_game))
    (:`then_5`
      (set `/Game/Blueprints/MySaveGame.MyNameVar` "Johnny" _asmy_save_game))
    (:`then_6`
      (set `/Game/Blueprints/MySaveGame.MyRotatorVar` (struct :`Pitch` 36.0 :`Yaw` 48.0 :`Roll` 12.0) _asmy_save_game))
    (:`then_7`
      (set `/Game/Blueprints/MySaveGame.MyTextVar` "This is the text var content!" _asmy_save_game))
    (:`then_8`
      (set `/Game/Blueprints/MySaveGame.MyVectorVar` (80.0 19.0 45.0) _asmy_save_game))
    (:`then_9`
      (set `/Game/Blueprints/MySaveGame.MyTransformVar` (`KismetMathLibrary.Conv_VectorToTransform` (`SceneComponent.K2_GetComponentLocation` (`self.DefaultSceneRoot`))) _asmy_save_game)
      (bind _returnvalue_3 (`CloudAPIFunctionLibrary.SaveGameToCloud` _output_get _asmy_save_game "foobarSaveKey")) ; Save the Game in the cloud
      (`KismetSystemLibrary.PrintText` (`KismetTextLibrary.Conv_StringToText` _returnvalue_3)))))

(event `self.ReceiveActorBeginOverlap`
  (params (OtherActor :type "Actor Object Reference")))

(event `self.ReceiveTick`
  (params (DeltaSeconds :type "Float (single-precision)")))

(fn `myStructTestFunc`
  (params (MyInputStruct :type "/Game/Structs/MySaveStruct Structure"))
  (returns (TheResult :type String))
  (return "foolala"))

(fn `UserConstructionScript`)